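; Player Blueprint that handles movement, fire input and the running animation state, and spawns a Gun on BeginPlay.
; Axis inputs move it along vectors built from control pitch only, with yaw zeroed, while left mouse and the Fire action both toggle a Firing flag.
; The Gun spawns at the capsule's RightHand socket transform without being attached.
; Tick prints velocity and sets IsRunning on PlayerAnims from the movement axes.
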(event `Key|LeftMouseButton`
  (params (Key :type "Key Structure"))
  ;[1 1 1] detect left mouse button down
  (:`Pressed`
    (set `self.Firing?` true))
  (:`Released`
    (set `self.Firing?` false)))

(event `self.ReceiveBeginPlay`
  ;[1 1 1] Spawn Gun
  (`|SpawnActorFromClass` "/Game/Blueprints/Gun.Gun_C" (`SceneComponent.GetSocketTransform` (`self.CapsuleComponent`) "RightHand" "RTS_World") "Undefined" "OverrideRootScale" null null))

(event `InputAxis|Forward/Back`
  (params (AxisValue :type "Float (single-precision)"))
  ;[1 1 1] Movement
  (`self.AddMovementInput` (`KismetMathLibrary.GetForwardVector` (`KismetMathLibrary.MakeRotator` 0.0 (.pitch (`self.GetControlRotation`)))) AxisValue))

(event `InputAction|Fire`
  (params (Key :type "Key Structure"))
  ;[1 1 1] Nothing
  (:`Pressed`
    (set `self.Firing?` true))
  (:`Released`
    (set `self.Firing?` false)))

(event `InputAxis|Left/Right`
  (params (AxisValue :type "Float (single-precision)"))
  ;[1 1 1] Movement
  (`self.AddMovementInput` (`KismetMathLibrary.GetRightVector` (`KismetMathLibrary.MakeRotator` 0.0 (.pitch (`self.GetControlRotation`)))) AxisValue))

(event `self.ReceiveTick`
  (params (DeltaSeconds :type "Float (single-precision)"))
  (bind _returnvalue (`SkeletalMeshComponent.GetAnimInstance` (`self.Mesh`)))
  (`KismetSystemLibrary.PrintString` (`KismetStringLibrary.Conv_VectorToString` (`self.GetVelocity`)))
  ;[1 1 1] Animations
  (`|ExecutionSequence`
    (:`then_0`
      (if (and (== (`self.GetInputAxisValue`) 0.0) (== (`self.GetInputAxisValue`) 0.0))
        (bind _asplayer_anims (cast `/Game/Blueprints/Player/Animations/PlayerAnims` _returnvalue))
        (set `/Game/Blueprints/Player/Animations/PlayerAnims.IsRunning?` false _asplayer_anims)
        (else
          (bind _asplayer_anims_2 (cast `/Game/Blueprints/Player/Animations/PlayerAnims` _returnvalue))
          (set `/Game/Blueprints/Player/Animations/PlayerAnims.IsRunning?` true _asplayer_anims_2))))))

(fn `UserConstructionScript`)