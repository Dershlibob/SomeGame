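; Top-down camera actor that follows the Player from a fixed height, looking straight down.
; On BeginPlay it sets its camera component to a square aspect ratio.
; Each Tick it looks up all Player actors and moves to the mesh's XY position plus half the velocity, so the view leads movement.
; There is no smoothing, and with several Players the last one found determines the position.
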(event `self.ReceiveBeginPlay`
  (`CameraComponent.SetAspectRatio` (`self.CameraComponent`) 1.0))

(event `self.ReceiveTick`
  (params (DeltaSeconds :type "Float (single-precision)"))
  (bind _outactors (`GameplayStatics.GetAllActorsOfClass` "/Game/Blueprints/Player/Player.Player_C"))
  (for _array_element _outactors
    (bind (_returnvalue_x _returnvalue_y) (`KismetMathLibrary.BreakVector` (`SceneComponent.K2_GetComponentLocation` (`Character.Mesh` _array_element))))
    (bind (_returnvalue_x_2 _returnvalue_y_2) (`KismetMathLibrary.BreakVector` (`self.GetVelocity` _array_element)))
    (`self.K2_SetActorLocationAndRotation` (`KismetMathLibrary.MakeVector` (+ _returnvalue_x (/ _returnvalue_x_2 2.0)) (+ _returnvalue_y (/ _returnvalue_y_2 2.0)) 1000.0) (struct :`Pitch` -90.0))))

(fn `UserConstructionScript`)