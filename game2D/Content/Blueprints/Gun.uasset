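; Gun actor that follows the Player's RightHand socket and fires Bullet actors toward the point under the mouse cursor.
; Every Tick it snaps to the socket, then checks the Player's Firing flag in semi-auto or automatic mode.
; Semi-auto uses a DoOnce reset on release, while automatic waits on CanSpawnBullet, re-armed from server world time after BulletInterval.
; Bullets spawn at the pawn's location, yawed toward the cursor hit.
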(event `self.ReceiveTick`
  (params (DeltaSeconds :type "Float (single-precision)"))
  (bind _returnvalue (`self.K2_GetActorLocation` (`GameplayStatics.GetPlayerPawn` 0)))
  (bind (_hitresult _returnvalue_2) (`PlayerController.GetHitResultUnderCursorByChannel` (`GameplayStatics.GetPlayerController` 0) "TraceTypeQuery1" true))
  (bind (_returnvalue_roll _returnvalue_pitch _returnvalue_yaw) (`KismetMathLibrary.BreakRotator` (`KismetMathLibrary.FindLookAtRotation` _returnvalue (`.Location` (`GameplayStatics.BreakHitResult` _hitresult)))))
  (`|ExecutionSequence`
    (:`then_0`
      ;[1 1 1] Position gun
      (bind _outactors (`GameplayStatics.GetAllActorsOfClass` "/Game/Blueprints/Player/Player.Player_C"))
      (for _array_element _outactors
        (`self.K2_SetActorTransform` (`SceneComponent.GetSocketTransform` (`Character.Mesh` _array_element) "RightHand" "RTS_World"))))
    (:`then_1`
      (if (`self.IsSemiAuto?`)
        ;[1 1 1] Conditions for semi auto
        (bind _outactors_2 (`GameplayStatics.GetAllActorsOfClass` "/Game/Blueprints/Player/Player.Player_C"))
        (for _array_element_2 _outactors_2
          (if (`/Game/Blueprints/Player/Player.Firing?` _array_element_2)
            (`/Engine/EditorBlueprintResources/StandardMacros.DoOnce` false :!label _label
              (:`Completed`
                ;[1 1 1] Spawn bullet
                (if _returnvalue_2 :!label _label_2
                  (set `self.CanSpawnBullet?` false)
                  (set `self.TimeFired` (`GameStateBase.GetServerWorldTimeSeconds` (`GameplayStatics.GetGameState`)))
                  (`|SpawnActorFromClass` "/Game/Blueprints/Bullet.Bullet_C" (`KismetMathLibrary.MakeTransform` _returnvalue (`KismetMathLibrary.MakeRotator` 0.0 0.0 _returnvalue_yaw)) "Undefined" "OverrideRootScale" null null)
                  (else
                    (`KismetSystemLibrary.PrintString` "Cursor clicked on nothing")))))
            (else
              (goto _label :!via `Reset`))))
        (else
          ;[1 1 1] Conditions for automatic
          (bind _outactors_3 (`GameplayStatics.GetAllActorsOfClass` "/Game/Blueprints/Player/Player.Player_C"))
          (for _array_element_3 _outactors_3
            (if (`/Game/Blueprints/Player/Player.Firing?` _array_element_3)
              (if (`self.CanSpawnBullet?`)
                (goto _label_2)))))))
    (:`then_2`
      ;[1 1 1] Calcs bullet interval
      (if (not (`self.CanSpawnBullet?`))
        (set `self.CanSpawnBullet?` (>= (- (`GameStateBase.GetServerWorldTimeSeconds` (`GameplayStatics.GetGameState`)) (`self.TimeFired`)) (`self.BulletInterval`)))))))

(fn `UserConstructionScript`)